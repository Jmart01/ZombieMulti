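; Zombie AI Blueprint that sends itself toward the nearest FPS_CharacterBase actor.
; On BeginPlay, a custom event gathers every FPS_CharacterBase, picks the closest and issues a single AIMoveTo through the AI controller with continuous goal tracking.
; Move success and failure only print debug strings, with no retargeting or retry.
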(event `FindBP_FPSCharacter`
  (bind _returnvalue_location (`KismetMathLibrary.BreakTransform` (`self.GetTransform` self)))
  (bind _outactors (`GameplayStatics.GetAllActorsOfClass` "/Script/ZombieMulti.FPS_CharacterBase"))
  (bind (_distance _returnvalue) (`GameplayStatics.FindNearestActor` _returnvalue_location _outactors))
  (bind _returnvalue_location_2 (`KismetMathLibrary.BreakTransform` (`self.GetTransform` _returnvalue)))
  (`AITask_MoveTo.AIMoveTo` (`AIBlueprintHelperLibrary.GetAIController` self) _returnvalue_location_2 _returnvalue -1.0 "Default" "Default" true true true
    (:`OnRequestFailed`
      (`KismetSystemLibrary.PrintString` "Fuck"))
    (:`OnMoveFinished`
      (`KismetSystemLibrary.PrintString` "YES!"))))

(event `self.ReceiveBeginPlay`
  (`self.FindBP_FPSCharacter`))

(fn `UserConstructionScript`)