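; BP_Spawner is a zombie spawner actor that calculates a per-round zombie count for the level.
; On BeginPlay it counts spawners and FPS characters, scaling the round total by players, zombies per player and round number.
; A loop raises and prints its in-scene counter up to its share, then increments the round after a delay.
; The delayed BP_ZombieAI spawn is disconnected, so no zombies actually spawn.
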(event `self.ReceiveBeginPlay`
  (bind _outactors (`GameplayStatics.GetAllActorsOfClass` "BP_Spawner_C"))
  (set `self.NumberOfSpawners` (`KismetArrayLibrary.Array_Length` _outactors))
  (bind _outactors_2 (`GameplayStatics.GetAllActorsOfClass` "/Script/ZombieMulti.FPS_CharacterBase"))
  (set `self.NumberOfPlayers` (`KismetArrayLibrary.Array_Length` _outactors_2))
  (`self.SpawnZombiesCalculation`))

(event `SpawnZombiesCalculation`
  (bind _output_get (set `self.ZombiesPerRound` (* (* (`self.NumberOfPlayers`) (`self.ZombiesPerPlayer`)) (`self.RoundNumber`))))
  (while (> (/ _output_get (`self.NumberOfSpawners`)) (`self.Zombies in scene`))
    (bind _output_get_2 (set `self.Zombies in scene` (+ (`self.Zombies in scene`) 1)))
    (`KismetSystemLibrary.PrintString` (`KismetStringLibrary.Conv_IntToString` _output_get_2)))
  (`KismetSystemLibrary.Delay` 5.0)
  (set `self.RoundNumber` (+ (`self.RoundNumber`) 1)))

(fn `UserConstructionScript`)